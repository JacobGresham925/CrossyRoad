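; FullTrainRev is an actor Blueprint, apparently a reverse-running train, that travels in a straight line and loops back to its starting point.
; BeginPlay stores the static mesh's world transform as the start.
; Each Tick moves the actor along the normalized Direction at Speed, scaled by delta time, without sweeping.
; Once the mesh's world Y drops to a hardcoded negative limit, the actor snaps back to the stored start.
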(event `self.ReceiveBeginPlay`
  (bind _output_get (set `self.Start` (`SceneComponent.K2_GetComponentToWorld` (`self.StaticMeshComponent`)))))

(event `self.ReceiveTick`
  (params (DeltaSeconds :type "Float (single-precision)"))
  (bind _location (.location (`SceneComponent.K2_GetComponentToWorld` (`self.StaticMeshComponent`))))
  (bind _output_get (set `self.Y>3000` (>= -15000.0 (.y _location))))
  (if _output_get
    (`self.K2_SetActorTransform` (stale `self.ReceiveBeginPlay` _output_get))
    (else
      (`self.K2_SetActorTransform` (`KismetMathLibrary.MakeTransform` (+ (* (`KismetMathLibrary.Normal` (`self.Direction`)) (* (`GameplayStatics.GetWorldDeltaSeconds`) (`self.speed`))) _location) (.rotation (`SceneComponent.K2_GetComponentToWorld` (`self.StaticMeshComponent`))) (.scale (`SceneComponent.K2_GetComponentToWorld` (`self.StaticMeshComponent`))))))))

(fn `UserConstructionScript`)